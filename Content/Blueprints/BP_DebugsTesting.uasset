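; Test actor for the RuntimeIMDebugsSubsystem runtime debug window, driving scene objects from its controls.
; BeginPlay shows the window, sets test brushes, registers a button, toggle, float field and spin box, then binds their change events.
; Handlers switch on control ID to spawn randomly placed cubes, set sphere hidden state, rotate an actor or offset the sphere along the cylinder-to-sphere direction.
; Tab and section creation calls are unconnected.
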(event Custom|OnButtonPressed_Event
  (params (ID :type Name))
  ;[0.15 0.15 0.15 0.5] Debug buttons
  (switch name ID
    (:AddCube
      (Game|SpawnActorfromClass (Variables|Default|GetCube) (Math|Transform|MakeTransform (Math|Random|RandomPointinBoundingBox (Transformation|GetActorLocation) "500.000000,500.000000,500.000000") "0, 0, 0" "1.000000,1.000000,1.000000") "AlwaysSpawn" "MultiplyWithRoot" 0 0))))

(event Custom|OnDebugFloatFieldChanged_Event
  (params (ID :type Name) (Value :type Float%20%28single-precision%29))
  ;[0.15 0.15 0.15 0.5] Debug Float fields
  (bind _output_get (Variables|Default|SetCurrentDebugFloatFieldValue Value))
  (switch name ID
    (:AddRotation
      (Class|Actor|AddActorWorldRotation (Variables|Default|GetActorToRotate) (Math|Rotator|MakeRotator 0.0 0.0 _output_get)))))

(event Custom|OnSliderChanged_Event
  (params (ID :type Name) (Value :type Float%20%28single-precision%29))
  ;[0.15 0.15 0.15 0.5] Debug Sliders
  (Variables|Default|SetCurrentSliderDebugValue Value)
  (switch name ID
    (:OffsetSphereCylinder
      (Transformation|SetActorLocation (Variables|Default|GetSphere) (+ (Variables|Default|GetSphereInitialLocation) (* (Math|Vector|Normalize (- (Transformation|GetActorLocation (Variables|Default|GetSphere)) (Transformation|GetActorLocation (Variables|Default|GetCylinder)))) (* (/ Value 1e+02) (Variables|Default|GetDistanceMaxOffset)))) false false))))

(event Custom|OnToggleChanged_Event
  (params (ID :type Name) (Value :type Boolean))
  ;[0.15 0.15 0.15 0.5] Debug Toggles
  (bind _output_get (Variables|Default|SetCurrentToggleDebugValue Value))
  (switch name ID
    (:ShowSphere
      (Rendering|SetActorHiddenInGame (Variables|Default|GetSphere) _output_get))))

(event EventBeginPlay
  (bind _returnvalue (Subsystems|GetRuntimeIMDebugsSubsystem))
  (bind _returnvalue_2 (Subsystems|GetRuntimeIMDebugsSubsystem))
  (bind _returnvalue_3 (Subsystems|GetRuntimeIMDebugsSubsystem))
  (Variables|Default|SetSphereInitialLocation (Transformation|GetActorLocation (Variables|Default|GetSphere)))
  (Class|RuntimeIMDebugsSubsystem|ShowWindow _returnvalue)
  (Variables|/Script/RuntimeIMDebugs.RuntimeIMDebugsSubsystem|SetTestBrush _returnvalue (Utilities|Struct|MakeSlateBrush (Utilities|Struct|MakeSlateColor "(R=0.208333,G=0.208333,B=0.208333,A=0.747826)" "UseColor_Specified") "Border" "NoTile" "NoMirror" "(X=32.000000,Y=32.000000)" (Utilities|Struct|MakeMargin 5.0 5.0 5.0 5.0) 0 "(CornerRadii=(X=0.000000,Y=0.000000,Z=0.000000,W=0.000000),Color=(SpecifiedColor=(R=0.000000,G=0.000000,B=0.000000,A=0.000000),ColorUseRule=UseColor_Specified),Width=0.000000,RoundingType=HalfHeightRadius,bUseBrushTransparency=False)"))
  (Variables|/Script/RuntimeIMDebugs.RuntimeIMDebugsSubsystem|SetTestBrush2 _returnvalue (Utilities|Struct|MakeSlateBrush (Utilities|Struct|MakeSlateColor "(R=0.000000,G=0.000000,B=0.000000,A=0.330435)" "UseColor_Specified") "Border" "NoTile" "NoMirror" "(X=32.000000,Y=32.000000)" (Utilities|Struct|MakeMargin 5.0 5.0 5.0 5.0) 0 "(CornerRadii=(X=0.000000,Y=0.000000,Z=0.000000,W=0.000000),Color=(SpecifiedColor=(R=0.000000,G=0.000000,B=0.000000,A=0.000000),ColorUseRule=UseColor_Specified),Width=0.000000,RoundingType=HalfHeightRadius,bUseBrushTransparency=False)"))
  (Class|RuntimeIMDebugsSubsystem|AddButton _returnvalue_3 "" "" "AddCube")
  (Class|RuntimeIMDebugsSubsystem|AddToggle _returnvalue_3 "" "None" "ShowSphere" "" false)
  (Class|RuntimeIMDebugsSubsystem|AddFloatField (Subsystems|GetRuntimeIMDebugsSubsystem) "SecondTab" "None" "AddRotation" "" 0.0)
  (Class|RuntimeIMDebugsSubsystem|AddSpinBox (Subsystems|GetRuntimeIMDebugsSubsystem) "SecondTab" "None" "OffsetSphereCylinder" "" 0.0 0.0 5e+02)
  (EventDispatchers|AssignOnButtonPressed _returnvalue_2 (EventDispatchers|CreateEvent :!event Custom|OnButtonPressed_Event))
  (EventDispatchers|AssignOnDebugFloatFieldChanged _returnvalue_2 (EventDispatchers|CreateEvent :!event Custom|OnDebugFloatFieldChanged_Event))
  (EventDispatchers|BindEventtoOnSpinBoxChanged _returnvalue_2 (EventDispatchers|CreateEvent :!event Custom|OnSliderChanged_Event))
  (EventDispatchers|AssignOnToggleChanged _returnvalue_2 (EventDispatchers|CreateEvent :!event Custom|OnToggleChanged_Event)))

(fn ConstructionScript)
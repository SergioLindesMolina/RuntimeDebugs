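; BP_DebugsTesting is a placeable test Blueprint for the runtime debug window provided by RuntimeIMDebugsSubsystem.
; On BeginPlay it shows the window and binds handlers for buttons, float fields, sliders (through the spin box delegate) and toggles.
; The float, slider and toggle handlers cache their latest value.
; Each handler switches on the control ID, with no cases wired yet, serving as a scaffold for debug actions.
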(event Custom|OnButtonPressed_Event
  (params (ID :type Name))
  ;[0.15 0.15 0.15 0.5] Debug buttons
  (switch name ID))

(event Custom|OnDebugFloatFieldChanged_Event
  (params (ID :type Name) (Value :type Float%20%28single-precision%29))
  ;[0.15 0.15 0.15 0.5] Debug Float fields
  (Variables|Debugs|SetCurrentDebugFloatFieldValue Value)
  (switch name ID))

(event Custom|OnSliderChanged_Event
  (params (ID :type Name) (Value :type Float%20%28single-precision%29))
  ;[0.15 0.15 0.15 0.5] Debug Sliders
  (Variables|Debugs|SetCurrentSliderDebugValue Value)
  (switch name ID))

(event Custom|OnToggleChanged_Event
  (params (ID :type Name) (Value :type Boolean))
  ;[0.15 0.15 0.15 0.5] Debug Toggles
  (Variables|Debugs|SetCurrentToggleDebugValue Value)
  (switch name ID))

(event EventBeginPlay
  (bind _returnvalue (Subsystems|GetRuntimeIMDebugsSubsystem))
  (Utilities|FlowControl|Sequence
    (:then_0
      (Class|RuntimeIMDebugsSubsystem|ShowWindow (Subsystems|GetRuntimeIMDebugsSubsystem))
      (EventDispatchers|AssignOnButtonPressed _returnvalue (EventDispatchers|CreateEvent :!event Custom|OnButtonPressed_Event))
      (EventDispatchers|AssignOnDebugFloatFieldChanged _returnvalue (EventDispatchers|CreateEvent :!event Custom|OnDebugFloatFieldChanged_Event))
      (EventDispatchers|BindEventtoOnSpinBoxChanged _returnvalue (EventDispatchers|CreateEvent :!event Custom|OnSliderChanged_Event))
      (EventDispatchers|AssignOnToggleChanged _returnvalue (EventDispatchers|CreateEvent :!event Custom|OnToggleChanged_Event)))))

(fn ConstructionScript)
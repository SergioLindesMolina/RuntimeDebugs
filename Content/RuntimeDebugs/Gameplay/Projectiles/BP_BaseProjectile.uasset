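; Base projectile, apparently fired by enemies, that is configured from a ProjectileData asset and damages characters it hits.
; Launch copies speed, gravity and homing settings to the ProjectileMovement component and aims at the target, with homing shots starting at unit speed.
; Mesh overlap ignores the owner, enemies and other projectiles, damages Characters and destroys the projectile.
; The construction script sets its lifespan from the same data.
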(event OnComponentBeginOverlap(StaticMesh)
  (params (OverlappedComponent :type Primitive%20Component%20Object%20Reference) (OtherActor :type Actor%20Object%20Reference) (OtherComp :type Primitive%20Component%20Object%20Reference) (OtherBodyIndex :type Integer) (bFromSweep :type Boolean) (SweepResult :type Hit%20Result%20Structure%20%28by%20ref%29))
  (if (Math|Boolean|ANDBoolean (!= OtherActor (Components|GetOwner)) (!= OtherActor self) (not (Class|GameplayStatics|ObjectIsA OtherActor "/Script/RuntimeDebugs.BaseEnemy")) (not (Class|GameplayStatics|ObjectIsA OtherActor "/Script/RuntimeDebugs.BaseProjectile")))
    (bind _ascharacter (Utilities|Casting|CastToCharacter OtherActor)
      (:then
        (bind _projectiledata (Variables|Default|GetProjectileData)
          (:then
            (Game|Damage|ApplyDamage _ascharacter (.Damage (Utilities|Struct|BreakProjectileInfo (Variables|/Script/RuntimeDebugs.ProjectileData|GetData _projectiledata))) 0 0)
            (Actor|DestroyActor))
          (:else)))
      (:CastFailed
        (Actor|DestroyActor)))))

(event Custom|Launch
  (params (Target :type Actor%20Object%20Reference))
  (bind _projectilemovement (Variables|Default|GetProjectileMovement))
  (bind _projectiledata (Variables|Default|GetProjectileData))
  (bind _data (Variables|/Script/RuntimeDebugs.ProjectileData|GetData _projectiledata))
  (bind (_homingprojectile _maxspeed) (Utilities|Struct|BreakProjectileInfo _data))
  (Variables|Default|SetTarget Target)
  (bind _projectiledata_2 (Variables|Default|GetProjectileData)
    (:then
      (Variables|/Script/Engine.ProjectileMovementComponent|SetMaxSpeed _projectilemovement (.MaxSpeed (Utilities|Struct|BreakProjectileInfo (Variables|/Script/RuntimeDebugs.ProjectileData|GetData _projectiledata_2))))
      (Variables|/Script/Engine.ProjectileMovementComponent|SetbIsHomingProjectile _projectilemovement (.HomingProjectile (Utilities|Struct|BreakProjectileInfo (Variables|/Script/RuntimeDebugs.ProjectileData|GetData _projectiledata_2))))
      (Variables|/Script/Engine.ProjectileMovementComponent|SetHomingAccelerationMagnitude _projectilemovement (.HomingAcceleration (Utilities|Struct|BreakProjectileInfo (Variables|/Script/RuntimeDebugs.ProjectileData|GetData _projectiledata_2))))
      (Variables|/Script/Engine.ProjectileMovementComponent|SetProjectileGravityScale _projectilemovement (.GravityScale (Utilities|Struct|BreakProjectileInfo (Variables|/Script/RuntimeDebugs.ProjectileData|GetData _projectiledata_2))))
      (Variables|/Script/Engine.ProjectileMovementComponent|SetHomingTargetComponent (Variables|Default|GetProjectileMovement) (Variables|/Script/Engine.Actor|GetRootComponent (Variables|Default|GetTarget)))
      (Variables|/Script/Engine.MovementComponent|SetVelocity (Variables|Default|GetProjectileMovement) (* (Math|Vector|GetUnitDirection(Vector) (Transformation|GetActorLocation) (Transformation|GetActorLocation (Variables|Default|GetTarget))) (select _homingprojectile 1.0 _maxspeed))))
    (:else)))

(fn ConstructionScript
  (bind _projectiledata (Variables|Default|GetProjectileData))
  (Utilities|IsValid _projectiledata
    (:Is%20Valid
      (Actor|SetLifeSpan (.lifetime (Variables|/Script/RuntimeDebugs.ProjectileData|GetData _projectiledata))))))
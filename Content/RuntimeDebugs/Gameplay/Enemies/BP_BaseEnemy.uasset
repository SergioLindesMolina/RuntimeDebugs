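; Base enemy that fires projectiles at Characters inside its attack-range sphere and shows a health bar until damage destroys it.
; The first overlap starts a looping cooldown timer that launches at a random target, stopping when none remain.
; Stats optionally copy from EnemyData into a runtime struct, with setters for max health, cooldown and range.
; A debug Fire handler triggers attacks, but its button registration is unwired.
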(event OnComponentBeginOverlap(Sphere)
  (params (OverlappedComponent :type Primitive%20Component%20Object%20Reference) (OtherActor :type Actor%20Object%20Reference) (OtherComp :type Primitive%20Component%20Object%20Reference) (OtherBodyIndex :type Integer) (bFromSweep :type Boolean) (SweepResult :type Hit%20Result%20Structure%20%28by%20ref%29))
  (bind _ascharacter (Utilities|Casting|CastToCharacter OtherActor))
  (bind _returnvalue (Utilities|Array|AddUnique (Variables|Default|GetPossibleTargets) _ascharacter))
  (if (== _returnvalue 0)
    (bind _returnvalue_2 (Utilities|Time|SetTimerbyFunctionName 0 "AttackPlayer" (Utilities|Struct|BreakEnemyInfo (Variables|Default|GetRuntimeEnemyData)) true))
    (Variables|Default|SetAttackTimerHandle _returnvalue_2)))

(event OnComponentEndOverlap(Sphere)
  (params (OverlappedComponent :type Primitive%20Component%20Object%20Reference) (OtherActor :type Actor%20Object%20Reference) (OtherComp :type Primitive%20Component%20Object%20Reference) (OtherBodyIndex :type Integer))
  (bind _attacktimerhandle (Variables|Default|GetAttackTimerHandle))
  (bind _ascharacter (Utilities|Casting|CastToCharacter OtherActor))
  (Utilities|Array|RemoveItem (Variables|Default|GetPossibleTargets) _ascharacter)
  (if (Utilities|Array|IsEmpty (Variables|Default|GetPossibleTargets))
    (if (Utilities|Time|IsValidTimerHandle _attacktimerhandle)
      (Utilities|Time|ClearandInvalidateTimerbyHandle _attacktimerhandle))))

(event Custom|AttackPlayer
  (bind _possibletargets (Variables|Default|GetPossibleTargets))
  (bind _returnvalue (Game|SpawnActorfromClass (Utilities|Struct|BreakEnemyInfo (Variables|Default|GetRuntimeEnemyData)) (Math|Transform|MakeTransform (Transformation|GetWorldLocation (Variables|Default|GetProjectileSpawnPoint)) "0, 0, 0" "1.000000,1.000000,1.000000") "Undefined" "MultiplyWithRoot" self 0))
  (bind _asbp_base_projectile (Utilities|Casting|CastToBP_BaseProjectile _returnvalue))
  (Utilities|IsValid _asbp_base_projectile
    (:Is%20Valid
      (Default|Launch _asbp_base_projectile (Utilities|Array|Get(acopy) _possibletargets (Math|Random|RandomIntegerinRange 0 (- (Utilities|Array|Length _possibletargets) 1)))))))

(event EventBeginPlay
  (Utilities|FlowControl|Sequence
    (:then_0
      ;[0.15 0.15 0.15 0.5] Runtime data
      (if (Variables|Default|GetbUseDefaultData)
        (Variables|Default|SetRuntimeEnemyData (Variables|/Script/RuntimeDebugs.EnemyData|GetData (Variables|Default|GetEnemyData)))))
    (:then_1
      (Variables|Default|SetCurrentHealth (Utilities|Struct|BreakEnemyInfo (Variables|Default|GetRuntimeEnemyData))))
    (:then_2
      (Components|Sphere|SetSphereRadius (Variables|Default|GetSphere) (Utilities|Struct|BreakEnemyInfo (Variables|Default|GetRuntimeEnemyData)) true))
    (:then_3
      (bind _aswbp_health_bar (Utilities|Casting|CastToWBP_HealthBar (UserInterface|GetWidget (Variables|Default|GetWidget))))
      (bind _output_get (Variables|Default|SetHealth%20Bar _aswbp_health_bar))
      (Default|Initialize _output_get (Variables|Default|GetCurrentHealth) (Utilities|Struct|BreakEnemyInfo (Variables|Default|GetRuntimeEnemyData))))
    (:then_4
      (|DebugGraph))))

(event Game|Damage|EventAnyDamage
  (params (Damage :type Float%20%28single-precision%29) (DamageType :type Damage%20Type%20Object%20Reference) (InstigatedBy :type Controller%20Object%20Reference) (DamageCauser :type Actor%20Object%20Reference))
  (Variables|Default|SetCurrentHealth (Math|Float|Clamp(Float) (- (Variables|Default|GetCurrentHealth) Damage) 0.0 (Utilities|Struct|BreakEnemyInfo (Variables|Default|GetRuntimeEnemyData))))
  (Default|UpdateHealth (Variables|Default|GetHealth%20Bar) (Variables|Default|GetCurrentHealth))
  ;[0.15 0 0 0.5] Kill
  (if (<= (Variables|Default|GetCurrentHealth) 0.0)
    (Actor|DestroyActor)
    (Utilities|Time|ClearandInvalidateTimerbyHandle (Variables|Default|GetAttackTimerHandle))))

(fn ConstructionScript
  (bind _enemydata (Variables|Default|GetEnemyData)
    (:then
      (Components|Sphere|SetSphereRadius (Variables|Default|GetSphere) (.attackrange (Variables|/Script/RuntimeDebugs.EnemyData|GetData _enemydata)) true))
    (:else)))

(fn UpdateMaxHealth
  (params (InMax%20Health :type Float%20%28single-precision%29))
  (bind _health_bar (Variables|Default|GetHealth%20Bar))
  (bind _structout (Utilities|Struct|SetmembersinEnemyInfo (Variables|Default|GetRuntimeEnemyData) InMax%20Health))
  (Utilities|IsValid _health_bar
    (:Is%20Valid
      (Default|UpdateMaxHealth _health_bar (.MaxHealth (Utilities|Struct|BreakEnemyInfo _structout))))))

(fn UpdateAttackCooldown
  (params (InAttack%20Cooldown :type Float%20%28single-precision%29))
  (Utilities|Struct|SetmembersinEnemyInfo (Variables|Default|GetRuntimeEnemyData) InAttack%20Cooldown))

(fn UpdateAttackRange
  (params (InAttack%20Range :type Float%20%28single-precision%29))
  (Utilities|Struct|SetmembersinEnemyInfo (Variables|Default|GetRuntimeEnemyData) InAttack%20Range)
  (Components|Sphere|SetSphereRadius (Variables|Default|GetSphere) (Utilities|Struct|BreakEnemyInfo (Variables|Default|GetRuntimeEnemyData)) true))

(event Custom|OnDebugButtonPressed
  (params (TabID :type Name) (SectionID :type Name) (ID :type Name))
  (switch name ID
    (:Fire
      (CallFunction|AttackPlayer))))
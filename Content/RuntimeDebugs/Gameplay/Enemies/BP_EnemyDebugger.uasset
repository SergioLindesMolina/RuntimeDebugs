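; Debug actor that exposes live tuning of the level's enemies in an "Enemies" tab of the RuntimeIMDebugs subsystem.
; On BeginPlay it gathers all BaseEnemy actors and builds a combo box to select one, plus spin boxes for attack cooldown, range and max health.
; Selection changes refresh the widgets, and edits call the selected enemy's update functions.
; Destroyed enemies leave the list, reselecting the first or resetting when none remain.
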(event Custom|RemoveEnemyFromList
  (params (DestroyedActor :type Actor%20Object%20Reference))
  ;[0.15 0.15 0.15 0.5] Remove the enemy when is destroyed from the list of enemies and from the list of the combo box
  (bind _asbase_enemy (Utilities|Casting|CastToBaseEnemy DestroyedActor))
  (Variables|Default|SetIndexToRemove (Utilities|Array|FindItem (Variables|Default|GetLevelEnemies) _asbase_enemy))
  (Utilities|Array|RemoveIndex (Variables|Default|GetLevelEnemies) (Variables|Default|GetIndexToRemove))
  (Class|RuntimeIMDebugsSubsystem|RemoveComboBoxOptionbyIndex (Subsystems|GetRuntimeIMDebugsSubsystem) "Enemies" "None" "LevelEnemies" (Variables|Default|GetIndexToRemove))
  (Utilities|FlowControl|Sequence
    (:then_0
      (if (== (Variables|Default|GetSelectedEnemy) _asbase_enemy)
        ;[0.15 0.15 0.15 0.5] If the destroyed enemy is the current selected put the index to 0
        (bind _succes (CallFunction|UpdateSelection))
        (if _succes
          (CallFunction|UpdateData (Variables|Default|GetSelectedEnemy))
          (Class|RuntimeIMDebugsSubsystem|SetComboBoxIndex (Subsystems|GetRuntimeIMDebugsSubsystem) "Enemies" "None" "LevelEnemies"))))
    (:then_1
      ;[0.15 0.15 0.15 0.5] If all enemies are destroyed reset data
      (CallFunction|ResetData))))

(event Custom|OnDebugComboBoxChanged_Event
  (params (TabID :type Name) (SectionID :type Name) (ID :type Name) (Index :type Integer))
  ;[0.15 0.15 0.15 0.5] When a combo box item is selected update the data and the enemy selected from the list of enemies
  (bind _succes (CallFunction|UpdateSelection Index))
  (if _succes
    (CallFunction|UpdateData (Variables|Default|GetSelectedEnemy))))

(event Custom|OnSpinBoxChanged
  (params (TabID :type Name) (SectionID :type Name) (ID :type Name) (Value :type Float%20%28single-precision%29))
  (bind _selectedenemy (Variables|Default|GetSelectedEnemy))
  ;[0.15 0.15 0.15 0.5] Change the enemy data
  (Utilities|IsValid _selectedenemy
    (:Is%20Valid
      (switch name ID
        (:AttackCooldown
          (Default|UpdateAttackCooldown _selectedenemy Value))
        (:AttackRange
          (Default|UpdateAttackRange _selectedenemy Value))
        (:MaxHealth
          (Default|UpdateMaxHealth _selectedenemy Value))))))

(event EventBeginPlay
  (bind _returnvalue (Subsystems|GetRuntimeIMDebugsSubsystem))
  (bind _returnvalue_2 (Subsystems|GetRuntimeIMDebugsSubsystem))
  (bind _returnvalue_3 (Subsystems|GetRuntimeIMDebugsSubsystem))
  (bind _selectedenemy (Variables|Default|GetSelectedEnemy))
  (bind _runtimeenemydata (Variables|/Game/RuntimeDebugs/Gameplay/Enemies/BP_BaseEnemy.BP_BaseEnemy_C|GetRuntimeEnemyData _selectedenemy))
  (Utilities|FlowControl|Sequence
    (:then_0
      ;[0.15 0.15 0.15 0.5] Get the list of enemies from the level
      (bind _outactors (Actor|GetAllActorsOfClass "/Script/RuntimeDebugs.BaseEnemy"))
      (Variables|Default|SetLevelEnemies _outactors)
      (for _array_element _outactors
        (Game|BindEventtoOnDestroyed _array_element (EventDispatchers|CreateEvent :!event Custom|RemoveEnemyFromList))))
    (:then_1
      ;[0.15 0.15 0.15 0.5] Select the first enemy from the list
      (CallFunction|UpdateSelection))
    (:then_2
      ;[0.15 0.15 0.15 0.5] Add the binding for the desired debug options types
      (EventDispatchers|AssignOnDebugComboBoxChanged _returnvalue_3 (EventDispatchers|CreateEvent :!event Custom|OnDebugComboBoxChanged_Event))
      (EventDispatchers|BindEventtoOnSpinBoxChanged _returnvalue_3 (EventDispatchers|CreateEvent :!event Custom|OnSpinBoxChanged))
      ;[0.15 0.15 0.15 0.5] Create the combo box from the list of enemies
      (bind _names (CallFunction|GenerateArrayOfNames (Variables|Default|GetLevelEnemies)))
      (Class|RuntimeIMDebugsSubsystem|AddComboBox (Subsystems|GetRuntimeIMDebugsSubsystem) "Enemies" "None" "LevelEnemies" "" _names)
      ;[0.15 0.15 0.15 0.5] Create the options that you want to change from the selected enemy
      (Class|RuntimeIMDebugsSubsystem|AddText _returnvalue_2 "Enemies" "None" "EnemyName" "" (Utilities|GetDisplayName _selectedenemy))
      (Class|RuntimeIMDebugsSubsystem|AddSpinBox _returnvalue_2 "Enemies" "None" "AttackCooldown" "" (.attackcooldown _runtimeenemydata) 0.0 2e+01)
      (Class|RuntimeIMDebugsSubsystem|AddSpinBox _returnvalue "Enemies" "None" "AttackRange" "" (.attackrange _runtimeenemydata) 0.0 2e+03)
      (Class|RuntimeIMDebugsSubsystem|AddSpinBox _returnvalue "Enemies" "None" "MaxHealth" "" (.maxhealth _runtimeenemydata) 0.0 1e+03))))

(fn ConstructionScript)

(fn UpdateSelection
  (params (InIndex :type Integer))
  (bind _levelenemies (Variables|Default|GetLevelEnemies))
  (if (and (Utilities|Array|IsValidIndex _levelenemies InIndex) (Utilities|Array|IsNotEmpty _levelenemies))
    (bind _asbp_base_enemy (Utilities|Casting|CastToBP_BaseEnemy (Utilities|Array|Get(acopy) (Variables|Default|GetLevelEnemies) InIndex)))
    (Variables|Default|SetSelectedEnemy _asbp_base_enemy)
    (return true)
    (else
      (Variables|Default|SetSelectedEnemy 0)
      (return false))))

(fn UpdateData
  (params (InEnemy :type BP%20Base%20Enemy%20Object%20Reference))
  (bind _returnvalue (Subsystems|GetRuntimeIMDebugsSubsystem))
  (bind _runtimeenemydata (Variables|/Game/RuntimeDebugs/Gameplay/Enemies/BP_BaseEnemy.BP_BaseEnemy_C|GetRuntimeEnemyData InEnemy))
  (Utilities|IsValid InEnemy
    (:Is%20Valid
      (Class|RuntimeIMDebugsSubsystem|SetText _returnvalue "Enemies" "None" "EnemyName" (Utilities|GetDisplayName InEnemy))
      (Class|RuntimeIMDebugsSubsystem|SetSpinBoxValue _returnvalue "Enemies" "None" "AttackCooldown" (.attackcooldown _runtimeenemydata))
      (Class|RuntimeIMDebugsSubsystem|SetSpinBoxValue _returnvalue "Enemies" "None" "AttackRange" (.attackrange _runtimeenemydata))
      (Class|RuntimeIMDebugsSubsystem|SetSpinBoxValue _returnvalue "Enemies" "None" "MaxHealth" (.maxhealth _runtimeenemydata)))))

(fn GenerateArrayOfNames
  (params (InActors :type Array%20of%20Actor%20Object%20References))
  (for _array_element InActors
    (Utilities|Array|Add (LocalVariables|GetLocalNames) (Utilities|GetDisplayName _array_element)))
  (return (LocalVariables|GetLocalNames)))

(fn ResetData
  (bind _returnvalue (Subsystems|GetRuntimeIMDebugsSubsystem))
  (if (Utilities|Array|IsEmpty (Class|RuntimeIMDebugsSubsystem|GetComboBoxOptions (Subsystems|GetRuntimeIMDebugsSubsystem) "Enemies" "None" "LevelEnemies"))
    (Class|RuntimeIMDebugsSubsystem|SetText _returnvalue "Enemies" "None" "EnemyName" "None")
    (Class|RuntimeIMDebugsSubsystem|SetSpinBoxValue _returnvalue "Enemies" "None" "AttackCooldown" 0.0)
    (Class|RuntimeIMDebugsSubsystem|SetSpinBoxValue _returnvalue "Enemies" "None" "AttackRange" 0.0)
    (Class|RuntimeIMDebugsSubsystem|SetSpinBoxValue _returnvalue "Enemies" "None" "MaxHealth" 0.0)))
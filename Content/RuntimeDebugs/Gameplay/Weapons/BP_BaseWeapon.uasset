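; BP_BaseWeapon is a base weapon Blueprint that deals damage on contact while its damage window is open.
; ActivateDamage and DeactivateDamage toggle that window and clear the list of actors already hit.
; Overlaps starting on DamageTrigger apply damage to damageable actors other than the weapon's owner, recording each so it is hit only once per activation.
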(event OnComponentBeginOverlap(DamageTrigger)
  (params (OverlappedComponent :type Primitive%20Component%20Object%20Reference) (OtherActor :type Actor%20Object%20Reference) (OtherComp :type Primitive%20Component%20Object%20Reference) (OtherBodyIndex :type Integer) (bFromSweep :type Boolean) (SweepResult :type Hit%20Result%20Structure%20%28by%20ref%29))
  (Utilities|IsValid OtherActor
    (:Is%20Valid
      (if (Math|Boolean|ANDBoolean (Variables|/Script/Engine.Actor|GetbCanBeDamaged OtherActor) (!= OtherActor (Components|GetOwner)) (Variables|Default|GetEnableDamage))
        (if (not (Utilities|Array|ContainsItem (Variables|Default|GetDamagedActors) OtherActor))
          (Game|Damage|ApplyDamage OtherActor (Variables|Default|GetDamage) 0 self)
          (Utilities|Array|AddUnique (Variables|Default|GetDamagedActors) OtherActor))))))

(event Custom|ActivateDamage
  (Variables|Default|SetEnableDamage true)
  (Utilities|Array|Clear (Variables|Default|GetDamagedActors)))

(event Custom|DeactivateDamage
  (Variables|Default|SetEnableDamage false)
  (Utilities|Array|Clear (Variables|Default|GetDamagedActors)))

(event EventBeginPlay)

(event Collision|EventActorBeginOverlap
  (params (OtherActor :type Actor%20Object%20Reference)))

(event EventTick
  (params (DeltaSeconds :type Float%20%28single-precision%29)))

(fn ConstructionScript)
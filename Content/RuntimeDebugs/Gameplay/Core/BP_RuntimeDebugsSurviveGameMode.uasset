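; Game mode for the RuntimeDebugs Survive level that tracks goal targets and announces level completion.
; On BeginPlay it gathers all BP_GoalTarget actors and binds to their completion events.
; Each completion scans the targets, breaking at an unfinished one, with the congratulations print following the loop.
; A DebugGraph registers a GameMode button through the RuntimeIMDebugs subsystem to complete all goals at once.
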(event Custom|OnGoalCompleted_Event
  (bind _array_element (Utilities|Array|ForEachLoopwithBreak (Variables|Default|GetGoalTargets))
    (:LoopBody
      (if (not (Default|IsGoalCompleted _array_element))
        (CallFunction|BreakCheckGoalLoop)))
    (:Completed
      (Development|PrintString "CONGRATULATIONS LEVEL COMPLETED" true true "(R=0.113101,G=1.000000,B=0.000000,A=1.000000)" 9999999999.0))))

(event Custom|Break_CheckGoalLoop
  (Utilities|Array|ForEachLoopwithBreak (Variables|Default|GetGoalTargets)) ; enters at Break
)

(event EventBeginPlay
  (Utilities|FlowControl|Sequence
    (:then_0
      (bind _outactors (Actor|GetAllActorsOfClass "/Game/RuntimeDebugs/Gameplay/Placeables/BP_GoalTarget.BP_GoalTarget_C"))
      (bind _output_get (Variables|Default|SetGoalTargets _outactors))
      (for _array_element _output_get
        (EventDispatchers|AssignOnGoalCompleted _array_element (delegate Custom|OnGoalCompleted_Event))))
    (:then_1
      (|DebugGraph))))

(fn ConstructionScript)

(event Custom|OnDebugButtonPressed
  (params (TabID :type Name) (SectionID :type Name) (ID :type Name))
  (switch name ID
    (:CompleteAllGoals
      (for _array_element (Variables|Default|GetGoalTargets)
        (Default|CompleteGoal _array_element)))))
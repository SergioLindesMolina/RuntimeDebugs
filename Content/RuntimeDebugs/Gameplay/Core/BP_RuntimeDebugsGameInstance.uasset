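; Game instance that builds a runtime debug menu for loading levels and tuning projectile data.
; Each world initialization runs DebugGraph, which binds RuntimeIMDebugs subsystem callbacks and adds a level picker, load button and per-projectile controls.
; Section IDs are asset names stripped of "DT_", which change handlers match to find the asset and edit its Data struct.
; That lookup prints every compared name on screen.
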(event EventOnWorldInitialized
  ;[0.15 0.15 0.15 0.5] Custom event that is call every time a world finish initializing, the call comes from FWorldDelegates::OnWorldInitializedActors
  (Utilities|FlowControl|Sequence
    (:then_1
      (|DebugGraph))))

(fn GetProjectileDatabyName
  (params (InData :type Array%20of%20Projectile%20Data%20Object%20References) (InName :type String))
  (for _array_element InData
    (Development|PrintString (.RightS (Utilities|String|Split (Utilities|GetDisplayName _array_element) "DT_")) true true "(R=0.000000,G=0.660000,B=1.000000,A=1.000000)" 5e+01)
    (Development|PrintString InName true true "(R=0.549204,G=1.000000,B=0.000000,A=1.000000)" 5e+01)
    (if (Utilities|Enum|Equal(Enum) InName (.RightS (Utilities|String|Split (Utilities|GetDisplayName _array_element) "DT_")))
      (LocalVariables|SetLocalFoundData _array_element)))
  (return (LocalVariables|GetLocalFoundData)))

(event Custom|OnSpinBoxChanged
  (params (TabID :type Name) (SectionID :type Name) (ID :type Name) (Value :type Float%20%28single-precision%29))
  (bind _returnvalue (Utilities|String|ToString(Name) SectionID))
  (bind _projectilesdata (Variables|Default|GetProjectilesData))
  (bind _founddata (CallFunction|GetProjectileDatabyName _projectilesdata _returnvalue))
  (switch name ID
    (:Damage
      (Utilities|IsValid _founddata
        (:Is%20Valid
          (Utilities|Struct|SetmembersinProjectileInfo (Variables|/Script/RuntimeDebugs.ProjectileData|GetData _founddata) Value))))
    (:LifeTime
      (Utilities|IsValid _founddata
        (:Is%20Valid
          (Utilities|Struct|SetmembersinProjectileInfo (Variables|/Script/RuntimeDebugs.ProjectileData|GetData _founddata) Value))))
    (:HommingAcceleration
      (Utilities|IsValid _founddata
        (:Is%20Valid
          (Utilities|Struct|SetmembersinProjectileInfo (Variables|/Script/RuntimeDebugs.ProjectileData|GetData _founddata) Value))))
    (:MaxSpeed
      (Utilities|IsValid _founddata
        (:Is%20Valid
          (Utilities|Struct|SetmembersinProjectileInfo (Variables|/Script/RuntimeDebugs.ProjectileData|GetData _founddata) Value))))
    (:GravityScale
      (Utilities|IsValid _founddata
        (:Is%20Valid
          (Utilities|Struct|SetmembersinProjectileInfo (Variables|/Script/RuntimeDebugs.ProjectileData|GetData _founddata) Value))))))

(event Custom|OnToggleChanged
  (params (TabID :type Name) (SectionID :type Name) (ID :type Name) (Value :type Boolean))
  (bind _returnvalue (Utilities|String|ToString(Name) SectionID))
  (bind _projectilesdata (Variables|Default|GetProjectilesData))
  (bind _founddata (CallFunction|GetProjectileDatabyName _projectilesdata _returnvalue))
  (switch name ID
    (:HommingProjectile
      (Utilities|IsValid _founddata
        (:Is%20Valid
          (Utilities|Struct|SetmembersinProjectileInfo (Variables|/Script/RuntimeDebugs.ProjectileData|GetData _founddata) Value))))))

(event Custom|OnDebugComboBoxSelected
  (params (TabID :type Name) (SectionID :type Name) (ID :type Name) (Index :type Integer))
  (switch name ID
    (:SelectLoadingLevel
      (Variables|Default|SetDebugLoadLevelIndex Index))))

(event Custom|OnDebugButtonPressed
  (params (TabID :type Name) (SectionID :type Name) (ID :type Name))
  (switch name ID
    (:LoadLevel
      (if (Utilities|Array|IsValidIndex (Variables|Default|GetLevelNames) (Variables|Default|GetDebugLoadLevelIndex))
        (Game|OpenLevel(byName) (Utilities|String|StringToName (Utilities|Array|Get(acopy) (Variables|Default|GetLevelNames) (Variables|Default|GetDebugLoadLevelIndex))))))))
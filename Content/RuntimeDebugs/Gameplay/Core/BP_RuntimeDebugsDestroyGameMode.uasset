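; Game mode for a RuntimeDebugs gameplay level where the player completes the level once every BaseEnemy is destroyed.
; On BeginPlay it gathers all BaseEnemy actors and binds their OnDestroyed, removing each from the list and printing a congratulations message when none remain.
; It also registers a kill-all-enemies button through RuntimeIMDebugsSubsystem, whose handler destroys the tracked enemies in reverse order as the list shrinks.
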(event Custom|OnDestroyed_Event
  (params (DestroyedActor :type Actor%20Object%20Reference))
  (bind _levelenemies (Variables|Default|GetLevelEnemies))
  (bind _returnvalue (Utilities|Array|IsEmpty _levelenemies))
  (bind _asbase_enemy (Utilities|Casting|CastToBaseEnemy DestroyedActor))
  (Utilities|Array|RemoveItem (Variables|Default|GetLevelEnemies) _asbase_enemy)
  (Development|PrintString (Utilities|String|ToString(Text) (Utilities|Text|FormatText "No more enemies {0}" _returnvalue)))
  (if _returnvalue
    (Development|PrintString "CONGRATULATIONS LEVEL COMPLETED" true true "(R=0.113101,G=1.000000,B=0.000000,A=1.000000)" 9999999999.0)))

(event EventBeginPlay
  (Utilities|FlowControl|Sequence
    (:then_0
      (bind _outactors (Actor|GetAllActorsOfClass "/Script/RuntimeDebugs.BaseEnemy"))
      (bind _output_get (Variables|Default|SetLevelEnemies _outactors))
      (for _array_element _output_get
        (Game|AssignOnDestroyed _array_element (delegate Custom|OnDestroyed_Event))))
    (:then_1
      (|DebugGraph))))

(fn ConstructionScript)

(event Custom|OnDebugButtonPressed
  (params (TabID :type Name) (SectionID :type Name) (ID :type Name))
  (switch name ID
    (:KillAllEnemies
      (bind _arrayelement (Utilities|Array|ReverseforEachLoop (Variables|Default|GetLevelEnemies))
        (:LoopBody
          (Utilities|IsValid _arrayelement
            (:Is%20Valid
              (Actor|DestroyActor _arrayelement))))))))